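; GA_Dash is a Gameplay Ability that launches the owning Character forward in a dash.
; On activation it commits, saves and zeroes ground friction, then applies a large velocity-change impulse along the actor's forward vector.
; It starts the AM_Dash montage with no logic on its callbacks, restores the saved friction and ends the ability.
; If the owner is not a Character, it ends right after committing.
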(event Ability|EventActivateAbility
  (Ability|CommitAbility)
  (bind _ascharacter (Utilities|Casting|CastToCharacter (Ability|GetOwningActorfromActorInfo))
    (:then
      (Variables|Default|SetGround%20Friction (Variables|/Script/Engine.CharacterMovementComponent|GetGroundFriction (Variables|/Script/Engine.Character|GetCharacterMovement _ascharacter)))
      (Variables|/Script/Engine.CharacterMovementComponent|SetGroundFriction (Variables|/Script/Engine.Character|GetCharacterMovement _ascharacter) 0.0)
      (Physics|AddImpulse (Variables|/Script/Engine.Character|GetCharacterMovement _ascharacter) (* (Transformation|GetActorForwardVector _ascharacter) 6e+03) true)
      (Animation|Montage|PlayMontage 0 "/Game/Blueprints/Characters/Animation/AM_Dash.AM_Dash"
        (:then
          _)
        (:OnCompleted
          _)
        (:OnBlendOut
          _)
        (:OnInterrupted
          _)
        (:OnNotifyBegin
          _)
        (:OnNotifyEnd
          _))
      (Variables|/Script/Engine.CharacterMovementComponent|SetGroundFriction (Variables|/Script/Engine.Character|GetCharacterMovement _ascharacter) (Variables|Default|GetGround%20Friction))
      (Ability|EndAbility))
    (:CastFailed
      (Ability|EndAbility))))

(event Ability|EventOnEndAbility
  (params (bWasCancelled :type Boolean)))