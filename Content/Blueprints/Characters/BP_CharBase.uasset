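; BP_CharBase is a character base Blueprint that uses the Gameplay Ability System for a sword melee attack.
; It acquires GA_Melee on BeginPlay, prints current Health, and activates the ability on MeleeAttack.
; Sword collider overlaps with exactly BP_Enemy send a Skill.Melee gameplay event to itself with the enemy as target.
; Die destroys the actor after a short delay; a not-self overlap check is left unconnected.
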(event OnComponentBeginOverlap(SwordCollider)
  (params (OverlappedComponent :type Primitive%20Component%20Object%20Reference) (OtherActor :type Actor%20Object%20Reference) (OtherComp :type Primitive%20Component%20Object%20Reference) (OtherBodyIndex :type Integer) (bFromSweep :type Boolean) (SweepResult :type Hit%20Result%20Structure%20%28by%20ref%29))
  (if (== (Utilities|GetClass OtherActor) "/Game/Blueprints/Characters/BP_Enemy.BP_Enemy_C")
    (Ability|SendGameplayEventtoActor self "(TagName=\"Skill.Melee\")" (Utilities|Struct|MakeGameplayEventData "(TagName=\"\")" 0 OtherActor))))

(event Custom|MeleeAttack
  (Abilities|TryActivateAbilitybyClass (Variables|Default|GetAbilitySystemComp) "/Game/Blueprints/GameplayAbilities/Melee/GA_Melee.GA_Melee_C" true))

(event EventBeginPlay
  (Class|CharBase|AcquireAbility "/Game/Blueprints/GameplayAbilities/Melee/GA_Melee.GA_Melee_C")
  (Development|PrintString (Utilities|String|ToString(Float) (.currentvalue (Variables|/Script/MagicBorn.AttributeSetBase|GetHealth (Variables|Default|GetAttributeSetBaseComp))))))

(event EventDie
  (Utilities|FlowControl|Delay 0.5)
  (Actor|DestroyActor))

(fn ConstructionScript)