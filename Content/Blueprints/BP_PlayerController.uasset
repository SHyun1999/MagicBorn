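; Player controller that creates the main HUD and routes player input to the controlled pawn.
; On BeginPlay it adds WBP_PrimaryUI to the viewport; look axes drive controller pitch and yaw, while move axes follow the camera's forward and right vectors.
; PrimaryAction triggers MeleeAttack and the HealthRegen action triggers TryDash, both through BP_CharBase casts.
; Jump casts to CharBase instead.
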(event EventBeginPlay
  (bind _returnvalue (UserInterface|CreateWidget "/Game/UI/Skills/WBP_PrimaryUI.WBP_PrimaryUI_C" self))
  (bind _output_get (Variables|Default|SetWBP_MainHUD _returnvalue))
  (UserInterface|Viewport|AddtoViewport _output_get 0))

(event Input|ActionEvents|InputActionJump
  (params (Key :type Key%20Structure :default "None"))
  ;[1 1 1] Movement
  (:Pressed
    (bind _aschar_base (Utilities|Casting|CastToCharBase (Pawn|GetControlledPawn)))
    (Character|Jump _aschar_base)))

(event Input|ActionEvents|InputActionHealthRegen
  (params (Key :type Key%20Structure :default "None"))
  (:Pressed
    (bind _asbp_char_base (Utilities|Casting|CastToBP_CharBase (Pawn|GetControlledPawn)))
    (Default|TryDash _asbp_char_base)))

(event Input|ActionEvents|InputActionPrimaryAction
  (params (Key :type Key%20Structure :default "None"))
  (:Pressed
    (bind _asbp_char_base (Utilities|Casting|CastToBP_CharBase (Pawn|GetControlledPawn)))
    (Default|MeleeAttack _asbp_char_base)))

(event Input|AxisEvents|InputAxisMoveForward
  (params (AxisValue :type Float%20%28single-precision%29))
  ;[1 1 1] Movement
  (Pawn|Input|AddMovementInput (Pawn|GetControlledPawn) (Math|Vector|GetForwardVector (Camera|GetCameraRotation (Game|GetPlayerCameraManager 0))) AxisValue false))

(event Input|AxisEvents|InputAxisMoveRight
  (params (AxisValue :type Float%20%28single-precision%29))
  ;[1 1 1] Movement
  (Pawn|Input|AddMovementInput (Pawn|GetControlledPawn) (Math|Vector|GetRightVector (Camera|GetCameraRotation (Game|GetPlayerCameraManager 0))) AxisValue false))

(event Input|AxisEvents|InputAxisLookUp
  (params (AxisValue :type Float%20%28single-precision%29))
  ;[1 1 1] Movement
  (Class|PlayerController|AddPitchInput AxisValue))

(event Input|AxisEvents|InputAxisLookRight
  (params (AxisValue :type Float%20%28single-precision%29))
  ;[1 1 1] Movement
  (Class|PlayerController|AddYawInput AxisValue))

(fn ConstructionScript)