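; Behavior tree task that sets a blackboard target to the player's controlled pawn.
; On AI execute it finds all BP_PlayerController actors and takes the pawn of the first one.
; A valid pawn is written to TargetKey and the task succeeds; an invalid pawn fails it.
; When no controller is found, the task never calls FinishExecute.
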(event EventReceiveExecuteAI
  (params (OwnerController :type AI%20Controller%20Object%20Reference) (ControlledPawn :type Pawn%20Object%20Reference))
  (bind _outactors (Actor|GetAllActorsOfClass "/Game/BP_PlayerController.BP_PlayerController_C"))
  (if (> (Utilities|Array|Length _outactors) 0)
    (Utilities|IsValid (Pawn|GetControlledPawn (Utilities|Array|Get(acopy) _outactors))
      (:Is%20Valid
        (Class|BTFunctionLibrary|SetBlackboardValueasObject (Variables|Default|GetTargetKey) (Pawn|GetControlledPawn (Utilities|Array|Get(acopy) _outactors)))
        (AI|BehaviorTree|FinishExecute true))
      (:Is%20Not%20Valid
        (AI|BehaviorTree|FinishExecute false)))))